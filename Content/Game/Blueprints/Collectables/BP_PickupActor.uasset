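; BP_PickupActor is a collectible pickup that rolls a random item type on the server at BeginPlay.
; The PickupType RepNotify spawns a CollectableItem at its transform: BP_ThrowableBomb for Bomb and Bomb Trap, BP_Shield for Recovery Kit and Shield.
; SetItem spawns a bomb for all four types.
; Collection logic that credits BP_BrawlPlayerState and destroys both actors is disconnected, and SpawnActorFromCollectable is an empty stub.
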(event Custom|SetItem
  (params (CollectibleType :type ECollectibles%20Enum :default "NewEnumerator4"))
  (switch Utilities|FlowControl|Switch|SwitchonECollectibles CollectibleType
    (:NewEnumerator0
      _)
    (:NewEnumerator1
      _)
    (:NewEnumerator2
      _)
    (:NewEnumerator3
      _))
  (Game|SpawnActorfromClass "/Game/Game/Blueprints/Collectables/BP_ThrowableBomb.BP_ThrowableBomb_C" (Transformation|GetActorTransform) "Undefined" 0 0))

(event EventBeginPlay
  (Networking|SwitchHasAuthority
    (:Authority
      (Variables|Default|SetPickupType (Utilities|Enum|ByteToEnumECollectibles (Math|Conversions|ToByte(Integer) (Math|Random|RandomIntegerinRange 1 4)))))))

(event Collision|EventActorBeginOverlap
  (params (OtherActor :type Actor%20Object%20Reference)))

(event EventTick
  (params (DeltaSeconds :type Float%20%28single-precision%29)))

(fn ConstructionScript)

(fn OnRepPickupType
  (bind _returnvalue (Transformation|GetActorTransform))
  (Development|PrintString "Setting collectable")
  (switch Utilities|FlowControl|Switch|SwitchonECollectibles (Variables|Default|GetPickupType)
    (:NewEnumerator0
      (bind _returnvalue_2 (Game|SpawnActorfromClass "/Game/Game/Blueprints/Collectables/BP_ThrowableBomb.BP_ThrowableBomb_C" _returnvalue "Undefined" 0 0 :!label _label))
      (Variables|Default|SetCollectableItem _returnvalue_2))
    (:NewEnumerator1
      (goto _label))
    (:NewEnumerator2
      (bind _returnvalue_3 (Game|SpawnActorfromClass "/Game/Game/Blueprints/Collectables/BP_Shield.BP_Shield_C" _returnvalue "Undefined" 0 0 :!label _label_2))
      (Variables|Default|SetCollectableItem _returnvalue_3))
    (:NewEnumerator3
      (goto _label_2))))

(fn SpawnActorfromCollectable
  (params (ActorType :type ECollectibles%20Enum :default "NewEnumerator4")))