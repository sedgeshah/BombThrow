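; BP_FakeBomb is a thrown bomb that explodes on a short timer and damages nearby pawns.
; Two multicast events launch its projectile movement, using either a supplied velocity or a suggested arc to a target point.
; Each duplicates the blast logic: effects, hiding, delayed cleanup, and a sphere trace sending BombHitMessage with distance-banded damage to unique actors.
; The sphere overlap event only checks authority, with nothing connected after it.
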(event OnComponentBeginOverlap(SphereCollision)
  (params (OverlappedComponent :type Primitive%20Component%20Object%20Reference) (OtherActor :type Actor%20Object%20Reference) (OtherComp :type Primitive%20Component%20Object%20Reference) (OtherBodyIndex :type Integer) (bFromSweep :type Boolean) (SweepResult :type Hit%20Result%20Structure%20%28by%20ref%29))
  (Networking|SwitchHasAuthority))

(event Custom|Multicast_ThrowToPoint
  (params (StartLocation :type Vector) (EndLocation :type Vector))
  (bind _projectilemovement (Variables|Default|GetProjectileMovement))
  (bind _sphere (Variables|Default|GetSphere))
  (bind _sphere_2 (Variables|Default|GetSphere))
  (bind _sphere_3 (Variables|Default|GetSphere))
  (bind _returnvalue (Transformation|GetWorldLocation _sphere_3))
  (bind _returnvalue_2 (Transformation|GetWorldLocation _sphere))
  (bind _returnvalue_3 (Transformation|GetWorldLocation _sphere_2))
  ;[1 1 1] Forward Throw
  ;;[1 1 1] Bomb explosion handling
  (bind _tossvelocity (Class|GameplayStatics|BlueprintSuggestProjectileVelocity StartLocation EndLocation 1.5e+03 0.0 "DoNotTrace" 0.0 false false))
  (Variables|/Script/Engine.MovementComponent|SetVelocity _projectilemovement _tossvelocity)
  (Components|Activation|Activate _projectilemovement false)
  (Utilities|FlowControl|Delay 0.5)
  (Audio|PlaySoundatLocation "/Game/StarterContent/Audio/Explosion_Cue.Explosion_Cue" _returnvalue_2 "0, 0, 0" 1.0 1.0 0.0 0 0 0 0)
  (Effects|SpawnEmitteratLocation "/Game/StarterContent/Particles/P_Explosion.P_Explosion" _returnvalue_2 "0, 0, 0" "2.000000,2.000000,2.000000")
  (Development|SetHiddeninGame _sphere true false)
  (Actor|SetLifeSpan 3.0)
  ;;[1 1 1] Handle bomb hit players (potentially environment actors/objects as well)
  (bind (_outhits _returnvalue_4) (Collision|MultiSphereTraceForObjects _returnvalue _returnvalue 4e+02 (Utilities|Array|MakeArray "ObjectTypeQuery3") false 0 "None"))
  (if _returnvalue_4
    (for _array_element _outhits
      (Utilities|Array|AddUnique (Variables|Default|GetDamagedActors) (.HitActor (Collision|BreakHitResult _array_element))))
    (for _array_element_2 (Variables|Default|GetDamagedActors)
      (Math|Float|CompareFloat (Math|Vector|Distance(Vector) _returnvalue_3 (Transformation|GetActorLocation _array_element_2)) 2.5e+02
        (:>
          (Math|Float|CompareFloat (Math|Vector|Distance(Vector) _returnvalue_3 (Transformation|GetActorLocation _array_element_2)) 4e+02
            (:==
              _)
            (:<
              _))
          (Class|BPICharacterEvents|BombHit(Message) _array_element_2 25.0 _returnvalue_3))
        (:==
          (Class|BPICharacterEvents|BombHit(Message) _array_element_2 5e+01 _returnvalue_3 :!label _label))
        (:<
          (Math|Float|CompareFloat (Math|Vector|Distance(Vector) _returnvalue_3 (Transformation|GetActorLocation _array_element_2)) 1e+02
            (:>
              (goto _label))
            (:==
              _)
            (:<
              _))
          (Class|BPICharacterEvents|BombHit(Message) _array_element_2 75.0 _returnvalue_3))))))

(event Custom|Multicast_IsThrownForward
  (params (ThrowVelocity :type Vector))
  (bind _sphere (Variables|Default|GetSphere))
  (bind _projectilemovement (Variables|Default|GetProjectileMovement))
  (bind _sphere_2 (Variables|Default|GetSphere))
  (bind _sphere_3 (Variables|Default|GetSphere))
  (bind _returnvalue (Transformation|GetWorldLocation _sphere_2))
  (bind _returnvalue_2 (Transformation|GetWorldLocation _sphere_3))
  (bind _returnvalue_3 (Transformation|GetWorldLocation _sphere))
  ;[1 1 1] Forward Throw
  ;;[1 1 1] Bomb explosion handling
  (Variables|/Script/Engine.MovementComponent|SetVelocity _projectilemovement ThrowVelocity)
  (Components|Activation|Activate _projectilemovement false)
  (Utilities|FlowControl|Delay 0.5)
  (Audio|PlaySoundatLocation "/Game/StarterContent/Audio/Explosion_Cue.Explosion_Cue" _returnvalue "0, 0, 0" 1.0 1.0 0.0 0 0 0 0)
  (Effects|SpawnEmitteratLocation "/Game/StarterContent/Particles/P_Explosion.P_Explosion" _returnvalue "0, 0, 0" "2.000000,2.000000,2.000000")
  (Development|SetHiddeninGame _sphere_2 true false)
  (Actor|SetLifeSpan 3.0)
  ;;[1 1 1] Handle bomb hit players (potentially environment actors/objects as well)
  (bind (_outhits _returnvalue_4) (Collision|MultiSphereTraceForObjects _returnvalue_2 _returnvalue_2 4e+02 (Utilities|Array|MakeArray "ObjectTypeQuery3") false 0 "None"))
  (if _returnvalue_4
    (for _array_element _outhits
      (Utilities|Array|AddUnique (Variables|Default|GetDamagedActors) (.HitActor (Collision|BreakHitResult _array_element))))
    (for _array_element_2 (Variables|Default|GetDamagedActors)
      (Math|Float|CompareFloat (Math|Vector|Distance(Vector) _returnvalue_3 (Transformation|GetActorLocation _array_element_2)) 2.5e+02
        (:>
          (Math|Float|CompareFloat (Math|Vector|Distance(Vector) _returnvalue_3 (Transformation|GetActorLocation _array_element_2)) 4e+02
            (:==
              _)
            (:<
              _))
          (Class|BPICharacterEvents|BombHit(Message) _array_element_2 25.0 _returnvalue_3))
        (:==
          (Class|BPICharacterEvents|BombHit(Message) _array_element_2 5e+01 _returnvalue_3 :!label _label))
        (:<
          (Math|Float|CompareFloat (Math|Vector|Distance(Vector) _returnvalue_3 (Transformation|GetActorLocation _array_element_2)) 1e+02
            (:>
              (goto _label))
            (:==
              _)
            (:<
              _))
          (Class|BPICharacterEvents|BombHit(Message) _array_element_2 75.0 _returnvalue_3))))))

(fn ConstructionScript)