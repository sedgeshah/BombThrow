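; Thrown bomb actor that sits at its landing point while a visual component flies there from the throwing character and explodes.
; The ThrowingCharacter RepNotify starts a Tick-driven rise above wall height, a curve-offset arc timed by distance, then an interpolated fall.
; On arrival it blinks, plays explosion effects and sphere-traces pawns, sending distance-tiered damage messages only to locally controlled ones.
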(event Custom|Enable_Move_To_Location
  ;[1 1 1] Setup
  (Transformation|SetWorldLocation (Variables|Default|GetBomb_Representation_SC) (Transformation|GetActorLocation (Variables|Default|GetThrowing_Character)) false true)
  (Rendering|SetVisibility (Variables|Default|GetBomb_Representation_SC) true true)
  (Variables|Default|SetMove_To_Location true)
  (Variables|Default|SetDistance_To_Parabola (Math|Vector|Distance(Vector) (Transformation|GetActorLocation (Variables|Default|GetThrowing_Character)) (Transformation|GetActorLocation)))
  (Variables|Default|SetVisual_Throw_Time (Math|Curves|GetFloatValue (Variables|Default|GetDistance_To_Time) (Variables|Default|GetDistance_To_Parabola)))
  (CallFunction|MaybeSwapIntoParabola)
  (if (Utilities|Enum|Equal(Enum) (Variables|Default|GetTravel_Phase) "NewEnumerator0")
    (Variables|Default|SetTravel_Phase "NewEnumerator1")))

(event Custom|Rise_Bomb
  (params (Delta_Time :type Float%20%28double-precision%29))
  (bind _bomb_representation_sc (Variables|Default|GetBomb_Representation_SC))
  (bind _returnvalue (Transformation|GetWorldLocation _bomb_representation_sc))
  ;[1 1 1] Rise
  (Transformation|SetWorldLocation (Variables|Default|GetBomb_Representation_SC) (Math|Vector|MakeVector (.x _returnvalue) (.y _returnvalue) (+ (* Delta_Time (Variables|Default|GetRise_Multiplier)) (.z _returnvalue))) false false)
  (CallFunction|MaybeSwapIntoParabola))

(event Custom|Parabola_Bomb
  (params (Delta_Time :type Float%20%28double-precision%29))
  ;[1 1 1] Parabola logic
  ;;[1 1 1] Update time
  (Variables|Default|SetCurrent_Visual_Throw_Time (Math|Float|Clamp(Float) (+ (Variables|Default|GetCurrent_Visual_Throw_Time) Delta_Time) 0.0 (Variables|Default|GetVisual_Throw_Time)))
  (Variables|Default|SetAlpha_Visual_Throw_Alpha (/ (Variables|Default|GetCurrent_Visual_Throw_Time) (Variables|Default|GetVisual_Throw_Time)))
  ;;[1 1 1] Update Parabola Location
  (Transformation|SetWorldLocation (Variables|Default|GetBomb_Representation_SC) (Math|Vector|MakeVector (.x (Math|Interpolation|Ease "Linear" (Variables|Default|GetAlpha_Visual_Throw_Alpha) (Variables|Default|GetParabola_Location) (Transformation|GetActorLocation))) (.y (Math|Interpolation|Ease "Linear" (Variables|Default|GetAlpha_Visual_Throw_Alpha) (Variables|Default|GetParabola_Location) (Transformation|GetActorLocation))) (+ (.z (Math|Interpolation|Ease "Linear" (Variables|Default|GetAlpha_Visual_Throw_Alpha) (Variables|Default|GetParabola_Location) (Transformation|GetActorLocation))) (Math|Curves|GetFloatValue (Variables|Default|GetParabola_Rise_Alpha_Curve) (Variables|Default|GetAlpha_Visual_Throw_Alpha)))) false false)
  ;;[1 1 1] Swap to falling
  (if (Math|Float|NearlyEqual(Float) (Variables|Default|GetAlpha_Visual_Throw_Alpha) 1.0 0.02)
    (Variables|Default|SetTravel_Phase "NewEnumerator3")))

(event Custom|Fall_Bomb
  (params (Delta_Time :type Float%20%28double-precision%29))
  ;[1 1 1] Fall logic
  (Transformation|SetWorldLocation (Variables|Default|GetBomb_Representation_SC) (Math|Interpolation|VInterpTo (Transformation|GetWorldLocation (Variables|Default|GetBomb_Representation_SC)) (Transformation|GetActorLocation) Delta_Time 1e+01) false true)
  (if (< (Math|Vector|Distance(Vector) (Transformation|GetWorldLocation (Variables|Default|GetBomb_Representation_SC)) (Transformation|GetActorLocation)) 1e+01)
    (Transformation|SetWorldLocation (Variables|Default|GetBomb_Representation_SC) (Transformation|GetActorLocation) false true)
    (CallFunction|BombExplode)
    (Variables|Default|SetTravel_Phase "NewEnumerator0")))

(event Custom|Maybe_Swap_Into_Parabola
  ;[1 1 1] Swap to Parabola
  (if (> (.z (Transformation|GetWorldLocation (Variables|Default|GetBomb_Representation_SC))) (CallFunction|MaxWallHeight))
    (Variables|Default|SetTravel_Phase "NewEnumerator2")
    (Variables|Default|SetParabola_Location (Transformation|GetWorldLocation (Variables|Default|GetBomb_Representation_SC)))))

(event Custom|BombExplode
  (bind _bomb (Variables|Default|GetBomb))
  (bind _bomb_2 (Variables|Default|GetBomb))
  (bind _bomb_3 (Variables|Default|GetBomb))
  (bind _returnvalue (Transformation|GetWorldLocation _bomb_3))
  (bind _returnvalue_2 (Transformation|GetWorldLocation _bomb_2))
  (bind _returnvalue_3 (Transformation|GetWorldLocation _bomb))
  (Rendering|Material|SetMaterial (Variables|Default|GetBomb) 0 "/Game/Assets/Bomb/M_Bomb_Beep.M_Bomb_Beep")
  (Utilities|FlowControl|Delay 0.1)
  (Rendering|Material|SetMaterial (Variables|Default|GetBomb) 0 "/Game/Assets/Bomb/M_Bomb_Base.M_Bomb_Base")
  (Utilities|FlowControl|Delay 0.1)
  (Rendering|Material|SetMaterial (Variables|Default|GetBomb) 0 "/Game/Assets/Bomb/M_Bomb_Beep.M_Bomb_Beep")
  (Utilities|FlowControl|Delay 0.1)
  (Audio|PlaySoundatLocation "/Game/StarterContent/Audio/Explosion01.Explosion01" _returnvalue_2 "0, 0, 0" 1.0 1.0 0.0 "/Game/StarterContent/Audio/Attn_BombSound.Attn_BombSound" 0 0 0)
  (Effects|SpawnEmitteratLocation "/Game/StarterContent/Particles/P_Explosion.P_Explosion" _returnvalue_2)
  (Camera|PlayWorldCameraShake "/Game/Game/Blueprints/Camera/BP_CameraShake.BP_CameraShake_C" _returnvalue_2 0.0 5e+04)
  (Development|SetHiddeninGame (Variables|Default|GetBomb) true true)
  (Actor|SetLifeSpan 3.0)
  (bind (_outhits _returnvalue_4) (Collision|MultiSphereTraceForObjects _returnvalue _returnvalue 1.5e+02 (Utilities|Array|MakeArray "ObjectTypeQuery3") false 0 "None"))
  (if _returnvalue_4
    (for _array_element _outhits
      (Utilities|Array|AddUnique (Variables|Default|GetDamaged_Actors) (.HitActor (Collision|BreakHitResult _array_element))))
    (for _array_element_2 (Variables|Default|GetDamaged_Actors)
      (if (Pawn|IsLocallyControlled (.AsPawn (Utilities|Casting|CastToPawn _array_element_2)))
        (Math|Float|CompareFloat (Math|Vector|Distance(Vector) _returnvalue_3 (Transformation|GetActorLocation _array_element_2)) 1e+02
          (:>
            (Math|Float|CompareFloat (Math|Vector|Distance(Vector) _returnvalue_3 (Transformation|GetActorLocation _array_element_2)) 1.5e+02
              (:==
                _)
              (:<
                _))
            (Class|BPICharacterEvents|BombHit(Message) _array_element_2 25 _returnvalue_3))
          (:==
            (Class|BPICharacterEvents|BombHit(Message) _array_element_2 35 _returnvalue_3 :!label _label))
          (:<
            (Math|Float|CompareFloat (Math|Vector|Distance(Vector) _returnvalue_3 (Transformation|GetActorLocation _array_element_2)) 5e+01
              (:>
                (goto _label))
              (:==
                _)
              (:<
                _))
            (Class|BPICharacterEvents|BombHit(Message) _array_element_2 45 _returnvalue_3)))))))

(event Custom|Swap_Textures
  (bind _bomb (Variables|Default|GetBomb))
  (Utilities|FlowControl|FlipFlop
    (:A
      (Rendering|Material|SetMaterial _bomb 0 "/Game/Assets/Bomb/M_Bomb_Beep.M_Bomb_Beep"))
    (:B
      (Rendering|Material|SetMaterial _bomb 0 "/Game/Assets/Bomb/M_Bomb_Base.M_Bomb_Base"))))

(event EventBeginPlay
  (Rendering|Material|SetMaterial (Variables|Default|GetBomb) 0 "/Game/Assets/Bomb/M_Bomb_Base.M_Bomb_Base"))

(event EventTick
  (params (DeltaSeconds :type Float%20%28single-precision%29))
  ;[1 1 1] Update travel phase
  (switch Utilities|FlowControl|Switch|SwitchonBomb_Travel_Phases (Variables|Default|GetTravel_Phase)
    (:NewEnumerator1
      (CallFunction|RiseBomb DeltaSeconds))
    (:NewEnumerator2
      (CallFunction|ParabolaBomb DeltaSeconds))
    (:NewEnumerator3
      (CallFunction|FallBomb DeltaSeconds)))
  ;[1 1 1] Debug
  (if false
    (Rendering|Debug|DrawDebugSphere (Transformation|GetWorldLocation (Variables|Default|GetBomb_Representation_SC)) 1e+01 5 (Utilities|Struct|MakeLinearColor 1.0 1.0 0.0 1.0) 1e+03 3.0)))

(fn ConstructionScript
  (Rendering|SetVisibility (Variables|Default|GetBomb_Representation_SC) false true))

(fn OnRepThrowingCharacter
  (Utilities|IsValid (Variables|Default|GetThrowing_Character)
    (:Is%20Valid
      (CallFunction|EnableMovetoLocation))))

(fn SwapMaterial)