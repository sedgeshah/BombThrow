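; Player state for a bomb-hurling brawl game, tracking the player's bomb count and shield in a PlayerStatus struct.
; CollectItem adds a bomb or grants the shield, then pushes the struct to the HUD inventory through the player controller.
; Server_ValidateBombUsage decrements the bomb count when above zero, without refreshing the HUD.
; BeginPlay caches a reference to player 0's character, which is otherwise unused.
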(event Custom|CollectItem
  (params (Item :type ECollectibles%20Enum :default "NewEnumerator4"))
  (bind _playerstatus (Variables|Default|GetPlayerStatus))
  (Development|PrintString "PlayerState: Collected Item")
  (switch Utilities|FlowControl|Switch|SwitchonECollectibles Item
    (:NewEnumerator0
      (Utilities|Struct|SetmembersinFPlayerStatus _playerstatus (+ (.Bombs (Utilities|Struct|BreakFPlayerStatus _playerstatus)) 1)))
    (:NewEnumerator3
      (Utilities|Struct|SetmembersinFPlayerStatus (Variables|Default|GetPlayerStatus) true)))
  (CallFunction|UpdatePlayerHUD))

(event Custom|Server_ValidateBombUsage
  (bind _playerstatus (Variables|Default|GetPlayerStatus))
  (Math|Integer|CompareInt (.bombs _playerstatus)
    (:>
      (Math|Integer|DecrementInt (.bombs _playerstatus)))))

(event EventBeginPlay
  (Variables|Default|SetBP_CharacterRef (.AsBP%20Bomb%20Hurl%20Character (Utilities|Casting|CastToBP_Bomb_Hurl_Character (Game|GetPlayerCharacter 0)))))

(fn ConstructionScript)

(fn UpdatePlayerHUD
  (Default|UpdateHUDInventory (.AsBP%20Hurler%20Player%20Controller (Utilities|Casting|CastToBP_HurlerPlayerController (Game|GetPlayerController))) (Variables|Default|GetPlayerStatus)))