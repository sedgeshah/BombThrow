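; Player controller for the bomb hurler game that sets up the player's camera, cursor and UI.
; On BeginPlay, after a short delay, it creates the HUD and popup widgets, shows the popup, blends to the top-down camera and flags the character as ready.
; StartMatch swaps to the HUD and enables movement.
; Helpers forward inventory updates, show popup messages and swap widgets by collapsing the current one.
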(event Custom|StartMatch
  (UIManagement|SwapWidgetto (Variables|Default|GetWBP_HudRef))
  (Variables|/Script/BombHurl.BombHurlCharacter|SetbCanPlayerMove (.AsBP%20Bomb%20Hurl%20Character (Utilities|Casting|CastToBP_Bomb_Hurl_Character (Game|GetPlayerCharacter 0))) true))

(event EventBeginPlay
  (Utilities|FlowControl|Delay 1.0)
  (Utilities|FlowControl|Sequence
    (:then_0
      (bind _returnvalue (Game|ConstructObjectfromClass "/Game/Game/Blueprints/UI/WBP_HUD.WBP_HUD_C"))
      (Variables|Default|SetWBP_HudRef _returnvalue)
      (bind _returnvalue_2 (Game|ConstructObjectfromClass "/Game/Game/Blueprints/UI/WBP_Popup.WBP_Popup_C"))
      (Variables|Default|SetWBP_PopUp _returnvalue_2)
      (UIManagement|SwapWidgetto _returnvalue_2))
    (:then_1
      (bind _outactors (Actor|GetAllActorsOfClass "/Game/Game/Blueprints/Camera/BP_TopDownCamera.BP_TopDownCamera_C"))
      (Game|Player|SetViewTargetwithBlend self (Utilities|Array|Get(acopy) _outactors) 0.5 "VTBlend_Linear" 0.0 false)
      (Utilities|FlowControl|Delay 1.25)
      (bind _asbp_bomb_hurl_character (Utilities|Casting|CastToBP_Bomb_Hurl_Character (Game|GetPlayerCharacter 0)))
      (Default|SetPlayerIsReady _asbp_bomb_hurl_character))
    (:then_2
      (bind _asbp_bomb_hurl_character_2 (Utilities|Casting|CastToBP_Bomb_Hurl_Character (Game|GetPlayerCharacter 0)))
      (Variables|Default|SetBP_CharRef _asbp_bomb_hurl_character_2))
    (:then_3
      (Input|SetInputModeGameandUI self 0 "DoNotLock" false)
      (Variables|Default|SetbShowMouseCursor true))))

(fn ConstructionScript)

(fn UpdateHUDInventory
  (params (PlayerInventory :type F%20Player%20Status%20Structure))
  (Default|UpdateInventory (Variables|Default|GetWBP_HudRef) PlayerInventory))

(fn SwapWidgetto
  (params (NextWidget :type User%20Widget%20Object%20Reference))
  (Utilities|IsValid (Variables|Default|GetCurrentWidget)
    (:Is%20Valid
      (Utilities|IsValid NextWidget
        (:Is%20Valid
          (Widget|SetVisibility (Variables|Default|GetCurrentWidget) "Collapsed"))))
    (:Is%20Not%20Valid
      _))
  (UserInterface|Viewport|AddtoViewport NextWidget 0)
  (Variables|Default|SetCurrentWidget NextWidget))

(fn ShowPopUp
  (params (MainMessage :type String) (AdditionalMessage :type String))
  (bind _wbp_popup (Variables|Default|GetWBP_PopUp))
  (Default|SetTextMessage _wbp_popup MainMessage AdditionalMessage)
  (if (not (== (Variables|Default|GetCurrentWidget) _wbp_popup))
    (UIManagement|SwapWidgetto _wbp_popup)))