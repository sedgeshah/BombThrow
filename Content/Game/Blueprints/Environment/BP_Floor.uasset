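; BP_Floor is a floor actor that generates its fence layout for a two-player match.
; GenerateFencing polls until two Pawns exist, then selects Fence1 and Fence2 in standard mode, or each of four fences at 50% odds otherwise.
; Once the GameState lists two players, a multicast event makes the selected fences visible and collidable.
; Older direct visibility and map-based approaches remain as disconnected nodes.
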(event Custom|GenerateFencing
  (bind _outactors (Actor|GetAllActorsOfClass "/Script/Engine.Pawn" :!label _label))
  (Math|Integer|CompareInt (Utilities|Array|Length _outactors) 2
    (:==
      (if (not (Variables|Default|GetbIsStandardMode))
        (Utilities|FlowControl|Sequence
          (:then_0
            (if (Math|Random|RandomBoolwithWeight 0.5)
              (Utilities|Array|Add (Variables|Default|GetVisibleMeshes) (Variables|Default|GetFence1))))
          (:then_1
            (if (Math|Random|RandomBoolwithWeight 0.5)
              (Utilities|Array|Add (Variables|Default|GetVisibleMeshes) (Variables|Default|GetFence2))))
          (:then_2
            (if (Math|Random|RandomBoolwithWeight 0.5)
              (Utilities|Array|Add (Variables|Default|GetVisibleMeshes) (Variables|Default|GetFence3))))
          (:then_3
            (if (Math|Random|RandomBoolwithWeight 0.5)
              (Utilities|Array|Add (Variables|Default|GetVisibleMeshes) (Variables|Default|GetFence4))))
          (:then_4
            (if (== (Utilities|Array|Length (Variables|/Script/Engine.GameStateBase|GetPlayerArray (Game|GetGameState))) 2) :!label _label_2
              (CallFunction|MulticastSetMeshVisibility (Variables|Default|GetVisibleMeshes))
              (else
                (Utilities|FlowControl|Delay 0.2)
                (goto _label_2)))))
        (else
          (Utilities|FlowControl|Sequence
            (:then_0
              (Utilities|Array|Add (Variables|Default|GetVisibleMeshes) (Variables|Default|GetFence1))
              (goto _label_2))
            (:then_1
              (Utilities|Array|Add (Variables|Default|GetVisibleMeshes) (Variables|Default|GetFence2))
              (goto _label_2))))))
    (:<
      (Utilities|FlowControl|Delay 0.05)
      (goto _label))))

(event Custom|Multicast_SetMeshVisibility
  (params (FenceRef :type Array%20of%20Static%20Mesh%20Component%20Object%20References))
  (for _array_element FenceRef
    (Development|SetHiddeninGame _array_element false false)
    (Collision|SetCollisionEnabled _array_element "QueryAndPhysics")
    (Rendering|SetVisibility _array_element true false)))

(fn ConstructionScript)

(fn OnRepBNotifyClients)