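; Actor that builds a square floor of attached tile actors on the server at BeginPlay, with a larger center tile at the midpoint.
; In procedural mode it randomly fills just under half the other cells, records each cell's occupancy in a Tiles map keyed by its indices, then calls OnFloorInitialised.
; Otherwise CreateGrid fills every other cell with standard floor tiles.
; ScanNeighbourhood is an unimplemented stub returning false.
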(event EventBeginPlay
  (bind _mesh_numbers_x (Variables|Default|GetMesh_Numbers_X))
  (Networking|SwitchHasAuthority
    (:Authority
      (Variables|Default|SetMesh_Numbers_Y _mesh_numbers_x)
      (Variables|Default|SetMidPoint (/ _mesh_numbers_x 2))
      (if (Variables|Default|GetbIsProcedural)
        (for _index (range 0 (- (Variables|Default|GetMesh_Numbers_X) 1))
          (for _index_2 (range 0 (- (Variables|Default|GetMesh_Numbers_Y) 1))
            (if (and (== _index (Variables|Default|GetMidPoint)) (== (Variables|Default|GetMidPoint) _index_2))
              (bind _returnvalue (Game|SpawnActorfromClass "/Game/Game/Blueprints/Environment/BP_CenterFloor.BP_CenterFloor_C" (Math|Transform|MakeTransform (Math|Vector|MakeVector (* _index (Variables|Default|GetMesh_Length)) (* _index_2 (Variables|Default|GetMesh_Width)) 0.0) (Transformation|GetActorRotation) "2.000000,2.000000,1.000000") "AlwaysSpawn" 0 0))
              (Transformation|AttachActorToActor _returnvalue self "None" "KeepRelative" "KeepWorld" "KeepRelative" true)
              (Utilities|Map|Add (Variables|Default|GetTiles) (Utilities|String|Append (Utilities|String|ToString(Integer) _index) (Utilities|String|ToString(Integer) _index_2)) true :!label _label)
              (elif (Math|Random|RandomBoolwithWeight 0.45)
                (bind _returnvalue_2 (Game|SpawnActorfromClass "/Game/Game/Blueprints/Environment/BP_Floor_Procedural.BP_Floor_Procedural_C" (Math|Transform|MakeTransform (Math|Vector|MakeVector (* _index (Variables|Default|GetMesh_Length)) (* _index_2 (Variables|Default|GetMesh_Width)) 0.0) (Transformation|GetActorRotation)) "AlwaysSpawn" 0 0))
                (Transformation|AttachActorToActor _returnvalue_2 self "None" "KeepRelative" "KeepWorld" "KeepRelative" true)
                (goto _label)
                (else
                  (Utilities|Map|Add (Variables|Default|GetTiles) (Utilities|String|Append (Utilities|String|ToString(Integer) _index) (Utilities|String|ToString(Integer) _index_2)) false))))))
        (Default|CallOnFloorInitialised)
        (else
          (CallFunction|CreateGrid))))))

(fn ConstructionScript)

(fn ScanNeighbourhood
  (params (Tiles :type Map%20of%20Strings%20to%20Booleans) (CurrentX :type Integer) (CurrentY :type Integer))
  (return false))

(fn CreateGrid
  (bind _midpoint (Variables|Default|GetMidPoint))
  (for _index (range 0 (- (Variables|Default|GetMesh_Numbers_X) 1))
    (for _index_2 (range 0 (- (Variables|Default|GetMesh_Numbers_Y) 1))
      (if (and (== _index _midpoint) (== _midpoint _index_2))
        (bind _returnvalue (Game|SpawnActorfromClass "/Game/Game/Blueprints/Environment/BP_CenterFloor.BP_CenterFloor_C" (Math|Transform|MakeTransform (Math|Vector|MakeVector (* _index (Variables|Default|GetMesh_Length)) (* _index_2 (Variables|Default|GetMesh_Width)) 0.0) (Transformation|GetActorRotation) "2.000000,2.000000,1.000000") "AlwaysSpawn" 0 0))
        (Transformation|AttachActorToActor _returnvalue self "None" "KeepRelative" "KeepWorld" "KeepRelative" true)
        (else
          (bind _returnvalue_2 (Game|SpawnActorfromClass "/Game/Game/Blueprints/Environment/BP_Floor.BP_Floor_C" (Math|Transform|MakeTransform (Math|Vector|MakeVector (* _index (Variables|Default|GetMesh_Length)) (* _index_2 (Variables|Default|GetMesh_Width)) 0.0) (Transformation|GetActorRotation)) "AlwaysSpawn" 0 0))
          (Transformation|AttachActorToActor _returnvalue_2 self "None" "KeepRelative" "KeepWorld" "KeepRelative" true))))))