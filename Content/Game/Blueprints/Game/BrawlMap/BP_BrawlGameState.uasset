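; Game state for the two-player Brawl map that starts and ends the match across server and clients.
; The server starts it by either counting ready registrations or polling both players' pawns until in game, then multicasts StartMatch to local controllers.
; On ending, it multicasts either the end-game HUD or a player-left popup that returns to the main menu.
; After a short delay, the server restarts the game through BP_BrawlGameMode.
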(event Custom|Multicast_EndDueToInterruption
  (bind _returnvalue (Class|GameplayStatics|GetPlayerControllerfromID))
  (bind _asbp_hurler_player_controller (Utilities|Casting|CastToBP_HurlerPlayerController _returnvalue))
  (Utilities|IsValid _asbp_hurler_player_controller
    (:Is%20Valid
      (Default|ShowPopUp _asbp_hurler_player_controller "One of players left." "Redirecting to main menu.")
      (Utilities|FlowControl|Delay 2.0)
      (Game|OpenLevel(byName) "MainMenu"))))

(event Custom|Server_EndGame
  (params (bIsDueToInterruption :type Boolean))
  (if bIsDueToInterruption
    (CallFunction|MulticastEndDuetoInterruption)
    (else
      (CallFunction|MulticastEndGamewithResult)))
  (Utilities|FlowControl|Delay 3.0)
  (Class|GameMode|RestartGame (.AsBP%20Brawl%20Game%20Mode (Utilities|Casting|CastToBP_BrawlGameMode (Game|GetGameMode)))))

(event Custom|Server_RegisterPlayerAsReady
  (params (SelfCharRef :type BP%20Bomb%20Hurl%20Character%20Object%20Reference))
  (Math|Integer|IncrementInt (Variables|Default|GetNumberOfPlayersReady)
    (:%20%20
      (CallFunction|ServerValidatePlayers))))

(event Custom|Multicast_StartMatch
  (Default|StartMatch (.AsBP%20Hurler%20Player%20Controller (Utilities|Casting|CastToBP_HurlerPlayerController (Game|GetPlayerController 0)))))

(event Custom|Server_CheckIfPlayersReady
  (bind _playerarray (Variables|Default|GetPlayerArray))
  (if (not (Variables|Default|GetbHasGameStarted))
    (Math|Integer|CompareInt (Utilities|Array|Length _playerarray) 2
      (:==
        (for _array_element _playerarray
          (bind _pawnprivate (Variables|/Script/Engine.PlayerState|GetPawnPrivate _array_element :!label _label)
            (:then
              (if (not (Variables|/Game/ThirdPerson/Blueprints/BP_Bomb_Hurl_Character.BP_Bomb_Hurl_Character_C|GetbIsInGame (.AsBP%20Bomb%20Hurl%20Character (Utilities|Casting|CastToBP_Bomb_Hurl_Character _pawnprivate)))) :!label _label_2
                (Utilities|FlowControl|Delay 0.05)
                (goto _label_2)))
            (:else
              (Utilities|FlowControl|Delay 0.05)
              (goto _label))))
        (Variables|Default|SetbHasGameStarted true)
        (CallFunction|MulticastStartMatch)
        (Variables|Default|SetNumberOfPlayersReady 0)))))

(event Custom|Server_ValidatePlayers
  (bind _numberofplayersready (Variables|Default|GetNumberOfPlayersReady))
  (Math|Integer|CompareInt _numberofplayersready 2
    (:==
      (Variables|Default|SetbHasGameStarted true)
      (Math|Integer|CompareInt (Utilities|Array|Length (Variables|Default|GetPlayerArray)) _numberofplayersready
        (:==
          (if (Variables|Default|GetbHasGameStarted)
            (CallFunction|MulticastStartMatch)))))))

(event Custom|Multicast_EndGameWithResult
  (if (not (Networking|IsDedicatedServer))
    (Default|ShowEndGameUI (Variables|/Game/Game/Blueprints/Player/BP_HurlerPlayerController.BP_HurlerPlayerController_C|GetWBP_HudRef (.AsBP%20Hurler%20Player%20Controller (Utilities|Casting|CastToBP_HurlerPlayerController (Class|GameplayStatics|GetPlayerControllerfromID)))))))

(event EventBeginPlay)

(event EventTick
  (params (DeltaSeconds :type Float%20%28single-precision%29)))

(fn ConstructionScript)