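; Game mode for the Brawl map that spawns players on procedural floor tiles and ends the game on logout.
; PostLogin stores the new controller and, while fewer than three players are present, spawns a BP_Bomb_Hurl_Character above random floor locations for it to possess.
; The floor-initialised event sets AllowSpawns, but only an unconnected delayed retry chain reads it or calls AssignControllers.
; Logout triggers ServerEndGame on BP_BrawlGameState.
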(event Custom|AllowSpawnPlayers
  (Variables|Default|SetbAllowSpawns true))

(event Custom|CheckSpawningAvailability
  (Math|Integer|CompareInt (Utilities|Array|Length (Variables|/Script/Engine.GameStateBase|GetPlayerArray (Game|GetGameState))) 3
    (:<
      (bind _outactors (Actor|GetAllActorsOfClass "/Game/Game/Blueprints/Environment/BP_Floor_Procedural.BP_Floor_Procedural_C"))
      (Development|PrintText (Utilities|Text|ToText(Integer) (Utilities|Array|Length _outactors)))
      (Variables|Default|SetFloors _outactors)
      (bind _returnvalue (Game|SpawnActorfromClass "/Game/ThirdPerson/Blueprints/BP_Bomb_Hurl_Character.BP_Bomb_Hurl_Character_C" (Math|Transform|MakeTransform (Math|Vector|MakeVector (.x (Transformation|GetActorLocation (Utilities|Array|Get(acopy) (Variables|Default|GetFloors) (Math|Random|RandomIntegerinRange 0 (- (Utilities|Array|Length _outactors) 1))))) (.y (Transformation|GetActorLocation (Utilities|Array|Get(acopy) (Variables|Default|GetFloors) (Math|Random|RandomIntegerinRange 0 (- (Utilities|Array|Length _outactors) 1))))) (+ (.z (Transformation|GetActorLocation (Utilities|Array|Get(acopy) (Variables|Default|GetFloors) (Math|Random|RandomIntegerinRange 0 (- (Utilities|Array|Length _outactors) 1))))) 1.5e+02)) "0, 0, 0" "1.000000,1.000000,1.000000") "Undefined" 0 0))
      (Pawn|Possess (Variables|Default|GetNextPC) _returnvalue))))

(event EventBeginPlay
  (bind _returnvalue (Actor|GetActorOfClass "/Game/Game/Blueprints/Environment/BP_ProcedurallyGeneratedFloor.BP_ProcedurallyGeneratedFloor_C"))
  (Development|PrintString (Utilities|GetDisplayName _returnvalue))
  (EventDispatchers|BindEventtoOnFloorInitialised _returnvalue (delegate Custom|AllowSpawnPlayers)))

(event EventTick
  (params (DeltaSeconds :type Float%20%28single-precision%29)))

(event EventPostLogin
  (params (NewPlayer :type Player%20Controller%20Object%20Reference))
  (Variables|Default|SetNextPC NewPlayer)
  (Math|Integer|CompareInt (Utilities|Array|Length (Variables|/Script/Engine.GameStateBase|GetPlayerArray (Game|GetGameState))) 3
    (:<
      (bind _outactors (Actor|GetAllActorsOfClass "/Game/Game/Blueprints/Environment/BP_Floor_Procedural.BP_Floor_Procedural_C"))
      (Development|PrintText (Utilities|Text|ToText(Integer) (Utilities|Array|Length _outactors)))
      (Variables|Default|SetFloors _outactors)
      (bind _returnvalue (Game|SpawnActorfromClass "/Game/ThirdPerson/Blueprints/BP_Bomb_Hurl_Character.BP_Bomb_Hurl_Character_C" (Math|Transform|MakeTransform (Math|Vector|MakeVector (.x (Transformation|GetActorLocation (Utilities|Array|Get(acopy) (Variables|Default|GetFloors) (Math|Random|RandomIntegerinRange 0 (- (Utilities|Array|Length _outactors) 1))))) (.y (Transformation|GetActorLocation (Utilities|Array|Get(acopy) (Variables|Default|GetFloors) (Math|Random|RandomIntegerinRange 0 (- (Utilities|Array|Length _outactors) 1))))) (+ (.z (Transformation|GetActorLocation (Utilities|Array|Get(acopy) (Variables|Default|GetFloors) (Math|Random|RandomIntegerinRange 0 (- (Utilities|Array|Length _outactors) 1))))) 1.5e+02)) "0, 0, 0" "1.000000,1.000000,1.000000") "Undefined" 0 0))
      (Pawn|Possess (Variables|Default|GetNextPC) _returnvalue))))

(event EventOnLogout
  (params (ExitingController :type Controller%20Object%20Reference))
  (Default|ServerEndGame (.AsBP%20Brawl%20Game%20State (Utilities|Casting|CastToBP_BrawlGameState (Game|GetGameState))) true))

(fn ConstructionScript)

(fn AssignControllers
  (for _array_element (Variables|/Script/Engine.GameStateBase|GetPlayerArray (Game|GetGameState))
    (bind _pawnprivate (Variables|/Script/Engine.PlayerState|GetPawnPrivate _array_element)
      (:then)
      (:else
        (Variables|Default|SetNextPC (.AsPlayer%20Controller (Utilities|Casting|CastToPlayerController (Pawn|GetController _pawnprivate))))
        (CallFunction|CheckSpawningAvailability)))))