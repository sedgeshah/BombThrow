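; Networked pickup actor that takes a random collectible type, such as bomb, bomb trap, recovery kit or shield, chosen by the server at BeginPlay.
; The type's RepNotify prints a debug message and spawns BP_ThirdPersonCharacter at the pickup's transform for all four listed types.
; Server-side sphere overlap clears the IsCollected gate and checks for a Pawn, but its type switch, SetItem and SpawnActorFromCollectible are unfinished stubs.
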(event OnComponentBeginOverlap(Sphere)
  (params (OverlappedComponent :type Primitive%20Component%20Object%20Reference) (OtherActor :type Actor%20Object%20Reference) (OtherComp :type Primitive%20Component%20Object%20Reference) (OtherBodyIndex :type Integer) (bFromSweep :type Boolean) (SweepResult :type Hit%20Result%20Structure%20%28by%20ref%29))
  (Networking|SwitchHasAuthority
    (:Authority
      (if (Variables|Default|GetbIsCollected)
        (Variables|Default|SetbIsCollected false)
        (Utilities|Casting|CastToPawn OtherActor)
        (switch Utilities|FlowControl|Switch|SwitchonECollectibles (Variables|Default|GetPickupType))))))

(event Custom|SetItem
  (params (CollectibleType :type ECollectibles%20Enum :default "NewEnumerator4"))
  (switch Utilities|FlowControl|Switch|SwitchonECollectibles CollectibleType))

(event EventBeginPlay
  (Networking|SwitchHasAuthority
    (:Authority
      (bind _output_get (Variables|Default|SetPickupType (Utilities|Enum|ByteToEnumECollectibles (Math|Conversions|ToByte(Integer) (Math|Random|RandomIntegerinRange 1 4))))))
    (:Remote
      (Utilities|FlowControl|Delay 0.2))))

(event Collision|EventActorBeginOverlap
  (params (OtherActor :type Actor%20Object%20Reference)))

(event EventTick
  (params (DeltaSeconds :type Float%20%28single-precision%29)))

(fn ConstructionScript)

(fn OnRepPickupType
  (Development|PrintString "Setting bomb")
  (switch Utilities|FlowControl|Switch|SwitchonECollectibles (Variables|Default|GetPickupType)
    (:NewEnumerator0
      _)
    (:NewEnumerator1
      _)
    (:NewEnumerator2
      _)
    (:NewEnumerator3
      _))
  (Game|SpawnActorfromClass "/Game/ThirdPerson/Blueprints/BP_ThirdPersonCharacter.BP_ThirdPersonCharacter_C" (Transformation|GetActorTransform) "Undefined" 0 0))

(fn SpawnActorfromCollectible
  (params (ActorType :type ECollectibles%20Enum :default "NewEnumerator4")))